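; Mirror portal actor that teleports the player to its paired mirror on overlap.
; It disables the pair's teleport to prevent bounce-back, and each mirror re-enables its own when the player stops overlapping it.
; The player keeps their offset from the mirror, while control yaw is reflected about this mirror's yaw and turned 180 degrees.
; After the move, it calls the player's ChangeCamera.
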(event Collision|EventActorBeginOverlap
  (params (OtherActor :type Actor%20Object%20Reference))
  (bind _pairmirror (Variables|Default|GetPairMirror))
  ;[1 1 1] If player entered the teleport area
  (if (Variables|Default|GetCanTeleport)
    (bind _asplayer (Utilities|Casting|CastToPlayer OtherActor))
    (Utilities|FlowControl|Sequence
      (:then_0
        ;[1 1 1] Prevents other mirror from teleporting the player back to this mirror
        (bind _asmirror (Utilities|Casting|CastToMirror _pairmirror))
        (Variables|/Game/Blueprints/Mirror.Mirror_C|SetCanTeleport _asmirror false)
        ;[1 1 1] Sets new position and new rotation
        (Transformation|SetActorLocation _asplayer (+ (Transformation|GetActorLocation _pairmirror) (- (Transformation|GetActorLocation _asplayer) (Transformation|GetActorLocation))) false true)
        (Pawn|SetControlRotation (Game|GetPlayerController 0) (Math|Rotator|MakeRotator (.roll (Transformation|GetActorRotation _asplayer)) (.pitch (Transformation|GetActorRotation _asplayer)) (+ (.yaw (Transformation|GetActorRotation _asplayer)) (* (- (.yaw (Transformation|GetActorRotation)) (.yaw (Transformation|GetActorRotation _asplayer))) 2.0) 1.8e+02))))
      (:then_1
        (Default|ChangeCamera _asplayer)))))

(event Collision|EventActorEndOverlap
  (params (OtherActor :type Actor%20Object%20Reference))
  ;[1 1 1] Enables teleport after player leaves the mirror
  (Utilities|Casting|CastToPlayer OtherActor)
  (Variables|Default|SetCanTeleport true))

(fn ConstructionScript)