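; Manager that tracks which mirror is nearest the player and gives that mirror's path to the Monster.
; From BeginPlay it finds the Monster, then rescans MirrorsWithPaths on a repeating Delay loop, calling UpdatePath only when the nearest index changes.
; Nearness weights horizontal and vertical distance with separate multipliers.
; DisableMirrors only sets the InMirror flag, which the scan does not read.
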(event EventBeginPlay
  ;[1 1 1] Searches for nearest mirror
  (Utilities|FlowControl|Sequence
    (:then_0
      (bind _returnvalue (Actor|GetActorOfClass "/Game/Blueprints/Monster/Monster.Monster_C"))
      (Variables|Default|SetMonster _returnvalue))
    (:then_1
      (Variables|Default|SetMinDistance 7.386721425538679e+18 :!label _label)
      (for (_array_element _array_index) (Variables|Default|GetMirrorsWithPaths)
        (bind _distance (CallFunction|DistancewithMultipliers (Transformation|GetActorLocation (Game|Player|GetPlayerPawn 0)) (Transformation|GetActorLocation _array_element)))
        (if (< _distance (Variables|Default|GetMinDistance))
          (Variables|Default|SetMinDistance _distance)
          (Variables|Default|SetCurrentNearest _array_index)))
      (if (!= (Variables|Default|GetCurrentNearest) (Variables|Default|GetNearestMirrorIndex))
        (Variables|Default|SetNearestMirrorIndex (Variables|Default|GetCurrentNearest))
        (Utilities|FlowControl|Sequence
          (:then_0
            (bind _asmirror (Utilities|Casting|CastToMirror (Utilities|Array|Get(acopy) (Variables|Default|GetMirrorsWithPaths) (Variables|Default|GetNearestMirrorIndex)))
              (:then
                (Default|UpdatePath (Variables|Default|GetMonster) (Variables|/Game/Blueprints/Mirror/Mirror.Mirror_C|GetPath _asmirror)))
              (:CastFailed
                (Variables|Default|SetNearestMirrorIndex -1))))
          (:then_1
            (Utilities|FlowControl|Delay (Variables|Default|GetDelayTime) :!label _label_2)
            (goto _label)))
        (else
          (goto _label_2))))))

(fn ConstructionScript)

(fn DisableMirrors
  (params (DisableRealMirrors :type Boolean))
  (Variables|Default|SetInMirror (not DisableRealMirrors)))

(fn DistancewithMultipliers
  (params (V1 :type Vector) (V2 :type Vector))
  (return (+ (* (Math|Vector|Distance(Vector) (Math|Vector|MakeVector (.x V1) (.y V1) 0.0) (Math|Vector|MakeVector (.x V2) (.y V2) 0.0)) (Variables|Default|GetHMultiplier)) (* (Math|Vector|Distance(Vector) (Math|Vector|MakeVector 0.0 0.0 (.z V1)) (Math|Vector|MakeVector 0.0 0.0 (.z V2))) (Variables|Default|GetVMultiplier)))))