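; Behavior tree task that advances a Monster's patrol index in the Blackboard, making it walk its PatrolPath back and forth.
; It steps the Index key up or down according to the DecrescentIndex flag and stores the result if it is valid in PatrolPath.
; When the step leaves the path, it flips the flag and retries in the opposite direction before finishing successfully.
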(event EventReceiveExecuteAI
  (params (OwnerController :type AI%20Controller%20Object%20Reference) (ControlledPawn :type Pawn%20Object%20Reference))
  (bind _decrescentindex (Variables|Default|GetDecrescentIndex))
  (if (Class|BTFunctionLibrary|GetBlackboardValueasBool (Variables|Default|GetDecrescentIndex))
    (Variables|Default|SetValueToBeAdded -1)
    (else
      (Variables|Default|SetValueToBeAdded 1)))
  (bind _asmonster (Utilities|Casting|CastToMonster ControlledPawn))
  (bind _output_get (Variables|Default|SetNewIndex (+ (Variables|Default|GetValueToBeAdded) (Class|BTFunctionLibrary|GetBlackboardValueasInt (Variables|Default|GetIndex)))))
  (if (Utilities|Array|IsValidIndex (Variables|/Game/Blueprints/Monster/Monster.Monster_C|GetPatrolPath _asmonster) _output_get)
    (Class|BTFunctionLibrary|SetBlackboardValueasInt (Variables|Default|GetIndex) (Variables|Default|GetNewIndex) :!label _label)
    (else
      (Class|BTFunctionLibrary|SetBlackboardValueasBool _decrescentindex (not (Class|BTFunctionLibrary|GetBlackboardValueasBool _decrescentindex)))
      (bind _output_get_2 (Variables|Default|SetValueToBeAdded (* (Variables|Default|GetValueToBeAdded) -1)))
      (bind _output_get_3 (Variables|Default|SetNewIndex (+ _output_get_2 (Class|BTFunctionLibrary|GetBlackboardValueasInt (Variables|Default|GetIndex)))))
      (if (Utilities|Array|IsValidIndex (Variables|/Game/Blueprints/Monster/Monster.Monster_C|GetPatrolPath _asmonster) _output_get_3)
        (goto _label)
        (else
          _))))
  (AI|BehaviorTree|FinishExecute true))