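; AI controller for the monster that runs its behavior tree on BeginPlay and reports sightings of the player.
; A successful AI Perception update on a Player sets CanSeePlayer on both the Blackboard and the controller.
; Losing perception leaves the flag set; ResetSight clears it and sets the Blackboard's Wait key.
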(event OnTargetPerceptionUpdated(AIPerception)
  (params (Actor :type Actor%20Object%20Reference) (Stimulus :type AI%20Stimulus%20Structure))
  (bind _bsuccessfullysensed (Utilities|Struct|BreakAIStimulus Stimulus))
  (Utilities|Casting|CastToPlayer Actor)
  (if _bsuccessfullysensed
    (AI|Components|Blackboard|SetValueasBool (Variables|Default|GetBlackboard) (Utilities|Name|MakeLiteralName "CanSeePlayer") _bsuccessfullysensed)
    (Variables|Default|SetCanSeePlayer _bsuccessfullysensed)))

(event EventBeginPlay
  (AI|RunBehaviorTree "/Game/Blueprints/Monster/Monter_BT.Monter_BT"))

(fn ConstructionScript)

(fn ResetSight
  (AI|Components|Blackboard|SetValueasBool (Variables|Default|GetBlackboard) (Utilities|Name|MakeLiteralName "Wait") true)
  (AI|Components|Blackboard|SetValueasBool (Variables|Default|GetBlackboard) (Utilities|Name|MakeLiteralName "CanSeePlayer") false)
  (Variables|Default|SetCanSeePlayer false))