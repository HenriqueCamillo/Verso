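; Behavior tree task that ends a monster's investigation of a heard sound once it reaches the spot.
; If the pawn is within a short distance of the blackboard SoundPosition, it waits briefly, then clears Investigating on the blackboard and on the Monster_AI controller.
; Otherwise it finishes successfully at once, leaving the state unchanged.
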(event EventReceiveExecuteAI
  (params (OwnerController :type AI%20Controller%20Object%20Reference) (ControlledPawn :type Pawn%20Object%20Reference))
  (if (< (Math|Vector|Distance(Vector) (Transformation|GetActorLocation ControlledPawn) (Class|BTFunctionLibrary|GetBlackboardValueasVector (Variables|Default|GetSoundPosition))) 45.0)
    (Utilities|FlowControl|Delay 2.0)
    (Class|BTFunctionLibrary|SetBlackboardValueasBool (Variables|Default|GetInvestigating) false)
    (bind _asmonster_ai (Utilities|Casting|CastToMonster_AI OwnerController))
    (Variables|/Game/Blueprints/Monster/Monster_AI.Monster_AI_C|SetInvestigating _asmonster_ai false))
  (AI|BehaviorTree|FinishExecute true))