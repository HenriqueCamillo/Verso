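; Monster is an AI-controlled enemy that drives adaptive music and follows a switchable patrol path.
; It binds to every Mirror's enter event, starting music outside the real world and stopping it on return.
; While music plays, Tick feeds player distance and sighting state into it and sets PlayerSpotted, cleared shortly after return so other scripts can read it.
; UpdatePath swaps the patrol path and resets the blackboard's index and direction.
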(event Custom|OnMirrorEnter
  (params (RealWorld :type Boolean))
  (bind _music (Variables|Default|GetMusic))
  ;[1 1 1] MusicLoop
  (if RealWorld
    (Class|FMODAudioComponent|SetParameter _music "State" 0.0)
    (Class|FMODAudioComponent|Stop _music)
    (Utilities|FlowControl|Delay 0.5) ; So that other scripts can know if player went back scared
    (Variables|Default|SetPlayerSpotted false)
    (else
      (Class|FMODAudioComponent|Play _music))))

(event EventBeginPlay
  (Utilities|FlowControl|Sequence
    (:then_0
      (bind _asmonster_ai (Utilities|Casting|CastToMonster_AI (AI|GetAIController self)))
      (Variables|Default|SetMonsterAI _asmonster_ai))
    (:then_1
      (bind _outactors (Actor|GetAllActorsOfClass "/Game/Blueprints/Mirror/Mirror.Mirror_C"))
      (for _array_element _outactors
        (EventDispatchers|BindEventtoOnMirrorEnter _array_element (delegate Custom|OnMirrorEnter))))))

(event EventTick
  (params (DeltaSeconds :type Float%20%28single-precision%29))
  (bind _music (Variables|Default|GetMusic))
  ;[1 1 1] MusicLoop
  (bind _returnvalue (Class|FMODAudioComponent|IsPlaying _music))
  (if _returnvalue
    (Class|FMODAudioComponent|SetParameter _music "Distance" (Math|Vector|Distance(Vector) (Transformation|GetActorLocation) (Transformation|GetActorLocation (Game|Player|GetPlayerPawn 0))))
    (if (Variables|/Game/Blueprints/Monster/Monster_AI.Monster_AI_C|GetCanSeePlayer (Variables|Default|GetMonsterAI))
      (Class|FMODAudioComponent|SetParameter _music "State" 1.0)
      (Variables|Default|SetPlayerSpotted true))))

(fn ConstructionScript)

(fn UpdatePath
  (params (Patrol%20Path :type Patrol%20Path%20Object%20Reference))
  (if (!= Patrol%20Path (Variables|Default|GetPath))
    (Variables|Default|SetPath Patrol%20Path)
    (bind _monsterai (Variables|Default|GetMonsterAI)
      (:then
        (Class|BlackboardComponent|SetValueasInt (Variables|/Script/AIModule.AIController|GetBlackboard _monsterai) (Utilities|Name|MakeLiteralName "PatrolPathIndex"))
        (AI|Components|Blackboard|SetValueasBool (Variables|/Script/AIModule.AIController|GetBlackboard _monsterai) (Utilities|Name|MakeLiteralName "DecrescentIndex") false))
      (:else))))