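; Behavior tree task for the Monster that picks its next patrol destination.
; It reads the Index blackboard value, offsets that point in the Monster's Path array by the path actor's location, and writes the result to PatrolPath.
; A missing or empty path falls back to the pawn's current location.
; An out-of-range index never calls FinishExecute, and the task does not change Index itself.
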(event EventReceiveExecuteAI
  (params (OwnerController :type AI%20Controller%20Object%20Reference) (ControlledPawn :type Pawn%20Object%20Reference))
  (bind _index (Variables|Default|GetIndex))
  (bind _patrolpath (Variables|Default|GetPatrolPath))
  (bind _returnvalue (Class|BTFunctionLibrary|GetBlackboardValueasInt _index))
  (bind _asmonster (Utilities|Casting|CastToMonster ControlledPawn))
  (bind _path (Variables|/Game/Blueprints/Monster/Monster.Monster_C|GetPath _asmonster)
    (:then
      (if (> (Utilities|Array|Length (Variables|/Game/Blueprints/Monster/PatrolPath.PatrolPath_C|GetPath _path)) 0)
        (if (Utilities|Array|IsValidIndex (Variables|/Game/Blueprints/Monster/PatrolPath.PatrolPath_C|GetPath _path) _returnvalue)
          (AI|BehaviorTree|SetBlackboardValueasVector _patrolpath (+ (Utilities|Array|Get(acopy) (Variables|/Game/Blueprints/Monster/PatrolPath.PatrolPath_C|GetPath _path) _returnvalue) (Transformation|GetActorLocation _path)))
          (AI|BehaviorTree|FinishExecute true))
        (else
          (AI|BehaviorTree|SetBlackboardValueasVector _patrolpath (Transformation|GetActorLocation ControlledPawn) :!label _label)
          (AI|BehaviorTree|FinishExecute true))))
    (:else
      (goto _label))))