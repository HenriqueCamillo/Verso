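; Inventory capture actor that renders a spinning 3D object through a SceneCaptureComponent2D, likely as an item preview.
; Every tick it advances the yaw of ObjectPivot at a constant, delta-time-scaled rate, then manually calls CaptureScene.
; Select toggles IsSelected and applies it as the capture component's visibility, while the rotation and capture calls run each tick regardless of that flag.
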(event Custom|Select
  (bind _output_get (Variables|Default|SetIsSelected (not (Variables|Default|GetIsSelected))))
  (Rendering|SetVisibility (Variables|Default|GetSceneCaptureComponent2D) _output_get false))

(event EventTick
  (params (DeltaSeconds :type Float%20%28single-precision%29))
  (bind _objectpivot (Variables|Default|GetObjectPivot))
  (bind _returnvalue (Transformation|GetWorldRotation _objectpivot))
  (bind (_roll _pitch _yaw) (Math|Rotator|BreakRotator _returnvalue))
  (Transformation|SetWorldRotation _objectpivot (Math|Rotator|MakeRotator _roll _pitch (+ (* DeltaSeconds 4e+01) _yaw)) false false)
  (Rendering|SceneCapture|CaptureScene (Variables|Default|GetSceneCaptureComponent2D) :!class /Script/Engine.SceneCaptureComponent2D))

(fn ConstructionScript)