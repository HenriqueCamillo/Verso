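; Post-process actor that gives the game a retro look with colour banding, dithering, optional cheap fog and optional downsampling.
; Construction Script sets rendering console variables and adds dynamic RGB or YUV retro and fog materials to the PostProcess.
; Vertical resolution goes to a material parameter collection at construction for preview and again on BeginPlay.
; At runtime, Tick polls viewport size when downsampling and updates r.ScreenPercentage on changes.
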(event EventBeginPlay
  (Actor|Tick|SetActorTickEnabled (Variables|Retro|GetbUseDownsample))
  (Utilities|FlowControl|Sequence
    (:then_0
      (CallFunction|SetGlobalMPC))
    (:then_1
      (if (and (Variables|Default|GetbMasterEnabled) (Variables|Retro|GetbUseDownsample))
        ;[0 1 0.364] Downsample functions; only processed at runtime
        (bind _breshaschanged (CallFunction|CheckforResolutionChange))
        (if _breshaschanged
          (CallFunction|SetDownsampleRes))))))

(event EventTick
  (params (DeltaSeconds :type Float%20%28single-precision%29))
  (if (and (Variables|Default|GetbMasterEnabled) (Variables|Retro|GetbUseDownsample))
    ;[0 1 0.364] Downsample functions; only processed at runtime
    (bind _breshaschanged (CallFunction|CheckforResolutionChange))
    (if _breshaschanged
      (CallFunction|SetDownsampleRes))))

(fn ConstructionScript
  (CallFunction|SetConsoleVars)
  (Variables|/Script/Engine.PostProcessComponent|SetbEnabled (Variables|Default|GetPostProcess) (Variables|Default|GetbMasterEnabled))
  (Utilities|FlowControl|Sequence
    (:then_0
      ;[0 0.6815 1] Create the retro material instance and apply it to post process
      (bind _returnvalue (Rendering|Material|CreateDynamicMaterialInstance (select (Variables|Retro|GetbUseYUVColourSpace) "/Game/Materials/PostProcess/PPI_RetroLookYUV.PPI_RetroLookYUV" "/Game/Materials/PostProcess/PPI_RetroLookRGB.PPI_RetroLookRGB") "None" :!class /Script/Engine.KismetMaterialLibrary))
      (bind _output_get (Variables|Retro|SetRetroLookRef _returnvalue))
      (Rendering|AddorUpdateBlendable (Variables|Default|GetPostProcess) _output_get 1.0 :!class /Script/Engine.PostProcessComponent)
      ;[1 0 0.1981] Set Post Process Parameters
      (Rendering|Material|SetScalarParameterValue (Variables|Retro|GetRetroLookRef) "ColourBanding" (Math|Conversions|ToFloat(Integer) (Variables|Retro|GetColourBands)) :!class /Script/Engine.MaterialInstanceDynamic)
      (Rendering|Material|SetScalarParameterValue (Variables|Retro|GetRetroLookRef) "DitherLerp" (Variables|Retro|GetDitheringStrength) :!class /Script/Engine.MaterialInstanceDynamic))
    (:then_1
      (if (Variables|Fogging|GetbEnableFog)
        ;[0 0.6815 1] Create the fog material instance and apply it to post process
        (bind _returnvalue_2 (Rendering|Material|CreateDynamicMaterialInstance "/Game/Materials/PostProcess/PP_CheapFog.PP_CheapFog" "None" :!class /Script/Engine.KismetMaterialLibrary))
        (bind _output_get_2 (Variables|Fogging|SetCheapFogInstance _returnvalue_2))
        (Rendering|AddorUpdateBlendable (Variables|Default|GetPostProcess) _output_get_2 1.0 :!class /Script/Engine.PostProcessComponent)
        ;[1 0 0.1981] Set Post Process Parameters
        (Rendering|Material|SetScalarParameterValue (Variables|Fogging|GetCheapFogInstance) "StartOffset" (Variables|Fogging|GetStartOffset) :!class /Script/Engine.MaterialInstanceDynamic)
        (Rendering|Material|SetScalarParameterValue (Variables|Fogging|GetCheapFogInstance) "FogDistance" (Variables|Fogging|GetFogDistance) :!class /Script/Engine.MaterialInstanceDynamic)
        (Rendering|Material|SetScalarParameterValue (Variables|Fogging|GetCheapFogInstance) "NoiseStrength" (Variables|Fogging|GetNoiseStrength) :!class /Script/Engine.MaterialInstanceDynamic)
        (Rendering|Material|SetScalarParameterValue (Variables|Fogging|GetCheapFogInstance) "NoiseScale" (Variables|Fogging|GetNoiseScale) :!class /Script/Engine.MaterialInstanceDynamic)
        (Rendering|Material|SetVectorParameterValue (Variables|Fogging|GetCheapFogInstance) "NoiseDirection" (Math|Conversions|ToLinearColor(Vector) (Variables|Fogging|GetNoiseDirection)) :!class /Script/Engine.MaterialInstanceDynamic)
        (Rendering|Material|SetVectorParameterValue (Variables|Fogging|GetCheapFogInstance) "FogColour" (Variables|Fogging|GetFogColour) :!class /Script/Engine.MaterialInstanceDynamic)))
    (:then_2
      (CallFunction|SetGlobalMPC))))

(fn CheckforResolutionChange
  (LocalVariables|SetbIsResSame (Math|Vector|Equal(Vector) (Variables|Internal|GetLastResolutionSize) (Viewport|GetViewportSize) 0.0001))
  (Variables|Internal|SetLastResolutionSize (Viewport|GetViewportSize))
  (return (not (LocalVariables|GetbIsResSame))))

(fn SetDownsampleRes
  (Development|ExecuteConsoleCommand (Utilities|String|Append "r.ScreenPercentage " (Utilities|String|ToString(Float) (* (Math|Float|Clamp(Float) (/ (Math|Conversions|ToFloat(Integer) (Math|Integer|Max(Integer) (Variables|Retro|GetDownsampleResolution) (Variables|Retro|GetFinalResolution))) (.Y (Math|Vector2D|BreakVector2D (Viewport|GetViewportSize))))) 1e+02))) 0)
  (return))

(fn SetConsoleVars
  (if (Variables|Default|GetbMasterEnabled)
    (Development|ExecuteConsoleCommand "r.PostProcessAAQuality 0" 0)
    (Development|ExecuteConsoleCommand "r.ShadowQuality 1" 0) ; This turns off shadow filtering
    (Development|ExecuteConsoleCommand "r.AmbientOcclusion.Compute.Smooth 0" 0)
    (else
      (Development|ExecuteConsoleCommand "r.PostProcessAAQuality 3" 0)
      (Development|ExecuteConsoleCommand "r.ShadowQuality 3" 0)
      (Development|ExecuteConsoleCommand "r.AmbientOcclusion.Compute.Smooth 1" 0)))
  ;[1 1 1] Only relevant for downsampling
  (if (and (Variables|Default|GetbMasterEnabled) (Variables|Retro|GetbUseDownsample))
    (Development|ExecuteConsoleCommand "r.upscale.quality 0" 0) ; https://docs.unrealengine.com/en-US/Engine/Rendering/ScreenPercentage/index.html
    (else
      (Development|ExecuteConsoleCommand "r.upscale.quality 3" 0))))

(fn SetGlobalMPC
  ;[0 1 0.1508] Set Global MPC Parameters
  ;
  ; (This has to be done in construction script for the viewport preview, AND on begin play so it actually works in game)
  (Rendering|Material|SetScalarParameterValue "/Game/Materials/MPC_RetroShaders.MPC_RetroShaders" "VerticalResolution" (Math|Conversions|ToFloat(Integer) (Math|Integer|Min(Integer) (Variables|Retro|GetDownsampleResolution) (Variables|Retro|GetFinalResolution))) :!class /Script/Engine.KismetMaterialLibrary)
  (return))