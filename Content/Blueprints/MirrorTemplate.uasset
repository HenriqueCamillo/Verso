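; Mirror actor that shows a simulated reflection through a paired mirror and doubles as a teleporter to it.
; Each tick it places the pair's SceneCaptureComponent2D from the reflected player-camera offset, with yaw mirrored using this actor's pitch.
; Player overlap moves them to the same relative position at the pair, mirrors control rotation and calls ChangeCamera.
; The pair's CanTeleport flag is cleared until the player exits, preventing bounce-back.
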(event EventTick
  (params (DeltaSeconds :type Float%20%28single-precision%29))
  (bind _returnvalue (Game|GetPlayerController 0))
  (bind _pairmirror (Variables|Default|GetPairMirror))
  (bind _defaultsceneroot (Variables|Default|GetDefaultSceneRoot))
  (bind _playercameramanager (Variables|/Script/Engine.PlayerController|GetPlayerCameraManager _returnvalue))
  (bind _transformcomponent (Variables|/Script/Engine.PlayerCameraManager|GetTransformComponent _playercameramanager))
  (bind _returnvalue_2 (Transformation|GetWorldRotation _transformcomponent))
  ;[1 1 1] Calculates and sets location and rotation of the camera of the pair mirror
  (Transformation|SetWorldLocationAndRotation (Actor|GetComponentbyClass _pairmirror "/Script/Engine.SceneCaptureComponent2D") (+ (* (Math|Vector|GetReflectionVector (- (Transformation|GetWorldLocation _defaultsceneroot) (Transformation|GetWorldLocation _transformcomponent)) (* (Math|Vector|GetForwardVector _defaultsceneroot) -1.0)) -1.0) (Transformation|GetWorldLocation (Variables|/Script/Engine.Actor|GetRootComponent _pairmirror))) (Math|Rotator|MakeRotator (.roll _returnvalue_2) (.pitch _returnvalue_2) (+ (.yaw _returnvalue_2) (* (- (.pitch (Transformation|GetActorRotation)) (.yaw _returnvalue_2)) 2.0) 1.8e+02)) false true))

(event Collision|EventActorBeginOverlap
  (params (OtherActor :type Actor%20Object%20Reference))
  (bind _pairmirror (Variables|Default|GetPairMirror))
  ;[1 1 1] If player entered the teleport area
  (if (Variables|Default|GetCanTeleport)
    (bind _asplayer (Utilities|Casting|CastToPlayer OtherActor))
    (Utilities|FlowControl|Sequence
      (:then_0
        ;[1 1 1] Prevents other mirror from teleporting the player back to this mirror
        (bind _asmirror_template (Utilities|Casting|CastToMirrorTemplate _pairmirror))
        (Variables|MirrorTemplate_C|SetCanTeleport _asmirror_template false)
        ;[1 1 1] Sets new position and new rotation
        (Transformation|SetActorLocation _asplayer (+ (Transformation|GetActorLocation _pairmirror) (- (Transformation|GetActorLocation _asplayer) (Transformation|GetActorLocation))) false true)
        (Pawn|SetControlRotation (Game|GetPlayerController 0) (Math|Rotator|MakeRotator (.roll (Transformation|GetActorRotation _asplayer)) (.pitch (Transformation|GetActorRotation _asplayer)) (+ (.yaw (Transformation|GetActorRotation _asplayer)) (* (- (.pitch (Transformation|GetActorRotation)) (.yaw (Transformation|GetActorRotation _asplayer))) 2.0) 1.8e+02))))
      (:then_1
        (Default|ChangeCamera _asplayer)))))

(event Collision|EventActorEndOverlap
  (params (OtherActor :type Actor%20Object%20Reference))
  ;[1 1 1] Enables teleport after player leaves the mirror
  (Utilities|Casting|CastToPlayer OtherActor)
  (Variables|Default|SetCanTeleport true))

(fn ConstructionScript)