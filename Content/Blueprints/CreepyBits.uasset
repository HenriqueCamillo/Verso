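; CreepyBits is an ambient audio Blueprint that plays its sound at irregular intervals, by its name for creepy atmosphere.
; BeginPlay sets a timer with a random delay between MinTime and MaxTime to call PlayCreepyBit.
; PlayCreepyBit plays the AudioComponent from the start and re-arms the timer with a fresh random delay, forming an endless loop without Tick.
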(event EventBeginPlay
  (Utilities|Time|SetTimerbyFunctionName 0 "PlayCreepyBit" (Math|Random|RandomFloatinRange (Variables|Default|GetMinTime) (Variables|Default|GetMaxTime))))

(fn ConstructionScript)

(fn PlayCreepyBit
  (Audio|Components|Audio|Play (Variables|Components|GetAudioComponent) 0.0)
  (Utilities|Time|SetTimerbyFunctionName 0 "PlayCreepyBit" (Math|Random|RandomFloatinRange (Variables|Default|GetMinTime) (Variables|Default|GetMaxTime))))