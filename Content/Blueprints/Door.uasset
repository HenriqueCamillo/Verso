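; Interactable door Blueprint that swings on a hinge and can be locked behind a required inventory item.
; When unlocked, interacting toggles the open state, playing or reversing a Timeline that drives the hinge's yaw.
; When locked, it asks the Player whether they hold the unlock item and clears the lock if so, without moving the door.
; Each interaction plays a sound chosen from the open or lock state.
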(event Custom|OnInteract
  (if (not (Variables|Default|GetisLocked))
    (Utilities|FlowControl|Sequence
      (:then_0
        ;[1 1 1] SetOpenCloseAudio
        (Audio|Components|Audio|SetSound (Variables|Default|GetAudio) (select (Variables|Default|GetisOpen) "/Game/Sound/Door_Open.Door_Open" "/Game/Sound/Door_Close.Door_Close"))
        (Audio|Components|Audio|Play (Variables|Default|GetAudio) 0.0 :!label _label))
      (:then_1
        ;[1 1 1] OpenOrClose
        (Variables|Default|SetisOpen (not (Variables|Default|GetisOpen)))
        (if (Variables|Default|GetisOpen)
          (bind _door_rotation (Timeline|DoorOpening Reverse)
            (:Update
              (Transformation|SetRelativeRotation (Variables|Default|GetHinge) (Math|Rotator|MakeRotator 0.0 0.0 _door_rotation) false false)))
          (else
            (Timeline|DoorOpening Play)))))
    (else
      (Utilities|FlowControl|Sequence
        (:then_0
          ;[1 1 1] Unlock
          (bind _asplayer (Utilities|Casting|CastToPlayer (Game|GetPlayerCharacter 0)))
          (bind _return (Default|CheckIteminInventory _asplayer (Variables|Default|GetItemToUnlock)))
          (Variables|Default|SetisLocked (not _return)))
        (:then_1
          ;[1 1 1] SetLockedUnlockAudio
          (Audio|Components|Audio|SetSound (Variables|Default|GetAudio) (select (Variables|Default|GetisLocked) "/Game/Sound/Door_Locked.Door_Locked" "/Game/Sound/Door_Lock.Door_Lock"))
          (goto _label))))))

(fn ConstructionScript)